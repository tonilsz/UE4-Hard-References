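; BP_Wall_Hard is a wall actor that takes its look from the player character when play begins.
; On BeginPlay it casts player 0's pawn to ThirdPersonCharacter and applies that character's logo material to the Decoration component.
; It then creates a dynamic instance of CubeMaterial, sets its BaseColor to the character's base color and assigns it to BaseMesh.
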(event `self.ReceiveBeginPlay`
  ;[1 1 1] Decoration
  (bind _asthird_person_character (cast `/Game/Practice/ThirdPersonCharacter` (`GameplayStatics.GetPlayerCharacter` 0)))
  (bind _newparam1 (`/Game/Practice/ThirdPersonCharacter.GetMaterialLogo` _asthird_person_character))
  (`PrimitiveComponent.SetMaterial` (`self.Decoration`) 0 _newparam1)
  ;[1 1 1] Base Colour
  (bind _newparam (`/Game/Practice/ThirdPersonCharacter.GetColorBase` _asthird_person_character))
  (bind _returnvalue (`KismetMaterialLibrary.CreateDynamicMaterialInstance` "/Game/Common/Geometry/Meshes/CubeMaterial.CubeMaterial"))
  (bind _output_get (set `self.MaterialInstance` _returnvalue))
  (`MaterialInstanceDynamic.SetVectorParameterValue` _output_get "BaseColor" _newparam)
  (`PrimitiveComponent.SetMaterial` (`self.BaseMesh`) 0 _output_get))

(fn `UserConstructionScript`)