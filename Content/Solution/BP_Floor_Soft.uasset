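; BP_Floor_Soft is a floor Blueprint that gives its static mesh a random material when play begins.
; On BeginPlay it picks a random row name from the Materials data table and looks up that row.
; When the row is found, it converts the Material field to an object and sets it on material slot zero.
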(event `self.ReceiveBeginPlay`
  (bind _materials (`self.materials`))
  (bind _outrownames (`DataTableFunctionLibrary.GetDataTableRowNames` _materials))
  (bind _returnvalue (`|GetDataTableRow` _materials (`|GetArrayItem` _outrownames (`KismetMathLibrary.RandomInteger` (+ (`KismetArrayLibrary.Array_LastIndex` _outrownames) 1))))
    (:`then`
      (`PrimitiveComponent.SetMaterial` (`self.StaticMesh`) 0 (`|ConvertAsset` (`.material_3_C8824FB94639ADCACA39E5842895AC81` (break `/Game/Solution/E_MaterialList_Soft` _returnvalue)))))))

(fn `UserConstructionScript`)